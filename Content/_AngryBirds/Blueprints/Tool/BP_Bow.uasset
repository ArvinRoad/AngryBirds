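; BP_Bow is the launcher actor for an Angry Birds-style game, still unfinished.
; On BeginPlay it spawns a Birdie_Sprite at the LaunchPotion component's location and stores it as Brid.
; Aim only reads the viewport mouse position; its clamped drag-to-velocity math and debug-drawn projectile path prediction are disconnected and never run.
; Launch is an empty stub.
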(event `self.ReceiveBeginPlay`
  (bind _returnvalue (`|SpawnActorFromClass` "/Game/_AngryBirds/Blueprints/Biology/Birdie_Sprite.Birdie_Sprite_C" (`KismetMathLibrary.Conv_VectorToTransform` (`SceneComponent.K2_GetComponentLocation` (`self.LaunchPotion`))) "Undefined" "OverrideRootScale" null null))
  (set `self.Brid` _returnvalue))

(fn `Aim`
  (locals (NewLocalVar_0 :type "Vector Structure" :default (0.0 0.0 0.0)))
  ;[1 1 1] 瞄准函数
  (bind _returnvalue (`WidgetLayoutLibrary.GetMousePositionOnViewport`)))

(fn `Launch`
  ;[1 1 1] 发射函数
)

(fn `UserConstructionScript`)