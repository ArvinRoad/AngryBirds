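; Player controller for an Angry Birds style game that turns touch input into slingshot aiming.
; On BeginPlay it sets the view to the level's BP_Camera and caches the BP_Bow actor.
; A touch press stores the viewport mouse position as the bow's clicked position and prints it for debugging.
; Touch movement calls the bow's Aim function, leaving the aiming logic to BP_Bow.
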(event `self.ReceiveBeginPlay`
  (bind _returnvalue (`GameplayStatics.GetActorOfClass` "/Game/_AngryBirds/Blueprints/Tool/BP_Camera.BP_Camera_C"))
  (`self.SetViewTargetWithBlend` _returnvalue)
  (bind _returnvalue_2 (`GameplayStatics.GetActorOfClass` "/Game/_AngryBirds/Blueprints/Tool/BP_Bow.BP_Bow_C"))
  (set `self.Bow` _returnvalue_2))

(event `InputTouch`
  (params (Location :type "Vector Structure") (FingerIndex :type "ETouchIndex Enum"))
  (:`Pressed`
    (bind _returnvalue (`WidgetLayoutLibrary.GetMousePositionOnViewport`))
    (bind _output_get (set `/Game/_AngryBirds/Blueprints/Tool/BP_Bow.ClickedPostion` _returnvalue (`self.Bow`)))
    (`KismetSystemLibrary.PrintString` (`KismetStringLibrary.Conv_Vector2dToString` _output_get)))
  (:`Moved`
    (`/Game/_AngryBirds/Blueprints/Tool/BP_Bow.Aim` (`self.Bow`))))

(fn `UserConstructionScript`)